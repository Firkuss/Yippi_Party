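; BP_Sniper is a turret trap that aims at the third-person character and shoots bullets.
; A detection sphere sets the target on overlap and clears it on exit, and Tick rotates the cube toward that target while detected.
; Entering also starts Fire, which spawns BP_Bullet at the arrow's transform in a FireRate-delayed loop.
; That loop has no exit condition, so firing continues after the character leaves.
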(event OnComponentBeginOverlap(Sphere)
  (params (OverlappedComponent :type Primitive%20Component%20Object%20Reference) (OtherActor :type Actor%20Object%20Reference) (OtherComp :type Primitive%20Component%20Object%20Reference) (OtherBodyIndex :type Integer) (bFromSweep :type Boolean) (SweepResult :type Hit%20Result%20Structure%20%28by%20ref%29))
  (bind _asbp_third_person_character (Utilities|Casting|CastToBP_ThirdPersonCharacter OtherActor))
  (Variables|Default|SetTarget _asbp_third_person_character)
  (Variables|Default|SetIs_Detect true)
  (CallFunction|Fire))

(event OnComponentEndOverlap(Sphere)
  (params (OverlappedComponent :type Primitive%20Component%20Object%20Reference) (OtherActor :type Actor%20Object%20Reference) (OtherComp :type Primitive%20Component%20Object%20Reference) (OtherBodyIndex :type Integer))
  (Utilities|Casting|CastToBP_ThirdPersonCharacter OtherActor)
  (Variables|Default|SetTarget 0)
  (Variables|Default|SetIs_Detect false))

(event Custom|Fire
  (Game|SpawnActorfromClass "/Game/GAME/Dev/Blueprints/Trap/BP_Bullet.BP_Bullet_C" (Transformation|GetWorldTransform (Variables|Default|GetArrow)) "AlwaysSpawn" "MultiplyWithRoot" 0 0 :!label _label)
  (Utilities|FlowControl|Delay (Variables|Default|GetFireRate))
  (goto _label))

(event EventTick
  (params (DeltaSeconds :type Float%20%28single-precision%29))
  (if (Variables|Default|GetIs_Detect)
    (Transformation|SetWorldRotation (Variables|Default|GetCube) (Math|Rotator|FindLookatRotation (Transformation|GetWorldLocation (Variables|Default|GetCube)) (Transformation|GetActorLocation (Variables|Default|GetTarget))) false false)))

(fn ConstructionScript)